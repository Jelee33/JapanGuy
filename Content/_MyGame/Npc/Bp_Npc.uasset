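; Customer NPC Blueprint that walks up to a table, shows an order slip for a random product and leaves by being destroyed on delivery.
; BeginPlay picks IstenenUrun from the first two product enum values, then HareketTimeline lerps the actor's transform from BaslangicNoktasi to MasaNoktasi without sweep.
; When the timeline finishes, the SiparisFisiWidget component becomes visible and displays the product through UrunuGoster.
; SiparisTeslimEdildi (order delivered) destroys the actor.
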(event Custom|SiparisTeslimEdildi
  (Actor|DestroyActor))

(event EventBeginPlay
  (Variables|Default|SetIstenenUrun (Utilities|Enum|ByteToEnumE_Uruntipi (Math|Conversions|ToByte(Integer) (Math|Random|RandomInteger 2))))
  (bind _alpha (Timeline|HareketTimeline Play)
    (:Update
      (bind _returnvalue (Math|Transform|Lerp(Transform) (Variables|Default|GetBaslangicNoktasi) (Variables|Default|GetMasaNoktasi) _alpha))
      (Transformation|SetActorTransform _returnvalue))
    (:Finished
      (Rendering|SetVisibility (Variables|Default|GetSiparisFisiWidget) true false)
      (bind _aswbp_siparis_fisi (Utilities|Casting|CastToWBP_SiparisFisi (UserInterface|GetUserWidgetObject (Variables|Default|GetSiparisFisiWidget))))
      (Default|UrunuGoster _aswbp_siparis_fisi (Variables|Default|GetIstenenUrun)))))

(fn ConstructionScript)